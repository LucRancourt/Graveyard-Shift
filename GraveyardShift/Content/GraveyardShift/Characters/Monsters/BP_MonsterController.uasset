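; BP_MonsterController is the AI controller that runs monsters, choosing a ghost or default navigation filter by pawn type.
; On BeginPlay it starts BT_Monster and stores a random exit from the monster's ExitTargets as the TargetExit blackboard key.
; Perception updates track repellents in range and drive the InRepellentRange key.
; CalculateRepelledRunDirection sums normalized vectors away from those repellents to give a combined flee direction.
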(event `self.ReceiveBeginPlay`
  (bind _asbp_monster (cast `/Game/GraveyardShift/Characters/Monsters/BP_Monster` (`self.K2_GetPawn`)))
  (bind _output_get (set `self.Monster` _asbp_monster))
  (`|ExecutionSequence`
    (:`then_0`
      (cast `/Game/GraveyardShift/Characters/Monsters/BP_Ghost` _output_get
        (:`then`
          (set `self.DefaultNavigationFilterClass` "/Game/GraveyardShift/Core/AI_Navigation/NavFilter_Ghost.NavFilter_Ghost_C"))
        (:`CastFailed`
          (set `self.DefaultNavigationFilterClass` "/Game/GraveyardShift/Core/AI_Navigation/NavFilter_MonsterDefault.NavFilter_MonsterDefault_C"))))
    (:`then_1`
      (`self.RunBehaviorTree` "/Game/GraveyardShift/Characters/Monsters/BT_Monster.BT_Monster")
      (`BlackboardComponent.SetValueAsObject` (`self.Blackboard`) (`self.TargetExit`) (`KismetArrayLibrary.Array_Random` (`/Game/GraveyardShift/Characters/Monsters/BP_Monster.ExitTargets` (`self.Monster`)))))))

(event `self.AIPerception.OnTargetPerceptionUpdated`
  (params (Actor :type "Actor Object Reference") (Stimulus :type "AIStimulus Structure"))
  (bind _repellantsinrange (`self.RepellantsInRange`))
  (bind _inrepellentrange (`self.InRepellentRange`))
  ; Repellant detection ~ detects any pickup for now
  (bind _asbp_repellent (cast `/Game/GraveyardShift/Core/AI_Navigation/BP_Repellent` Actor))
  (if Stimulus_bSuccessfullySensed
    (`KismetSystemLibrary.PrintString` (`KismetSystemLibrary.GetDisplayName` _asbp_repellent))
    (`KismetArrayLibrary.Array_AddUnique` (`self.RepellantsInRange`) _asbp_repellent)
    (`BlackboardComponent.SetValueAsBool` (`self.Blackboard`) _inrepellentrange true)
    (else
      (`KismetSystemLibrary.PrintString` "DONT SEE")
      (`KismetArrayLibrary.Array_RemoveItem` _repellantsinrange _asbp_repellent)
      (`BlackboardComponent.SetValueAsBool` (`self.Blackboard`) _inrepellentrange (> (`KismetArrayLibrary.Array_Length` _repellantsinrange) 0)))))

(fn `CalculateRepelledRunDirection`
  (returns (RunDirection :type "Vector Structure"))
  (locals (MonsterPawn :type "Pawn Object Reference") (RunDir :type "Vector Structure" :default (0.0 0.0 0.0)))
  (set `local.MonsterPawn` (`self.K2_GetPawn`))
  (for _array_element (`self.RepellantsInRange`)
    (set `local.RunDir` (+ (`local.RunDir`) (`KismetMathLibrary.Vector_Normal2D` (- (`self.K2_GetActorLocation` (`local.MonsterPawn`)) (`self.K2_GetActorLocation` _array_element))))))
  (return (`KismetMathLibrary.Normal` (`local.RunDir`))))

(fn `UserConstructionScript`)