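; Undead monster character that rises out of the ground when spawned, then becomes AI-controlled.
; BeginPlay drops it 600 units, and a timeline scaled by RiseDuration lifts it back.
; When finished, it enables capsule collision and gravity, then spawns and possesses with BP_UndeadController.
; Each tick, SpriteLookAt yaws the sprite plane between actor forward and the camera axis by LookAtAlpha, using a dot product to handle rear views.
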(event `self.ReceiveBeginPlay`
  (bind _returnvalue (`self.K2_GetActorLocation`))
  ; Set StartingPosition Values
  (set `self.TargetLocation` _returnvalue)
  (bind _output_get (set `self.SpawnedLocation` (- _returnvalue (* (`self.GetActorUpVector`) 600.0))))
  (`self.K2_SetActorLocation` _output_get false true)
  ; Rising
  (set `self.bIsRising` true)
  (`TimelineComponent.SetPlayRate` (`self.Rising_Timeline`) (`KismetMathLibrary.SafeDivide` 1.0 (`self.RiseDuration`)))
  (bind (_direction _rising_floattrack) (`Timeline|Rising_Timeline` :!via `PlayFromStart`)
    (:`Update`
      (`self.K2_SetActorLocation` (`KismetMathLibrary.VLerp` (`self.SpawnedLocation`) (`self.TargetLocation`) _rising_floattrack)))
    (:`Finished`
      (set `self.bIsRising` false)
      (`self.SetupUndeadForController`))))

(event `self.ReceiveTick`
  (params (DeltaSeconds :type "Float (single-precision)"))
  (`self.SpriteLookAt`))

(fn `SetupUndeadForController`
  (`|ExecutionSequence`
    (:`then_0`
      ; Character/Capsule
      (`PrimitiveComponent.SetCollisionEnabled` (`self.CapsuleComponent`) "QueryAndPhysics")
      (set `CharacterMovementComponent.GravityScale` 1.0 (`self.CharacterMovement`)))
    (:`then_1`
      ; AI Controller
      (bind _returnvalue (`|SpawnActorFromClass` "/Game/GraveyardShift/Characters/Monsters/BP_UndeadController.BP_UndeadController_C" (`KismetMathLibrary.MakeTransform` (0.0 0.0 0.0)) "Undefined" "MultiplyWithRoot" null null))
      (`Controller.Possess` _returnvalue self))))

(fn `SpriteLookAt`
  (bind _returnvalue (`self.K2_GetActorLocation`))
  (bind _returnvalue_2 (`self.K2_GetActorLocation`))
  (bind _lookatalpha (`self.LookAtAlpha`))
  (bind (_relativerotation_roll _relativerotation_pitch) (`KismetMathLibrary.BreakRotator` (`SceneComponent.RelativeRotation` (`self.Plane`))))
  (bind _returnvalue_3 (`KismetMathLibrary.FindLookAtRotation` _returnvalue_2 (+ _returnvalue_2 (`self.GetActorForwardVector`))))
  (bind _returnvalue_4 (`KismetMathLibrary.Normal` (- (`PlayerCameraManager.GetCameraLocation` (`GameplayStatics.GetPlayerCameraManager` 0)) _returnvalue_2)))
  (bind (_returnvalue_roll _returnvalue_pitch _returnvalue_yaw) (`KismetMathLibrary.BreakRotator` (`KismetMathLibrary.RLerp` _returnvalue_3 (`KismetMathLibrary.FindLookAtRotation` _returnvalue (+ _returnvalue _returnvalue_4)) _lookatalpha true)))
  (bind (_returnvalue_roll_2 _returnvalue_pitch_2 _returnvalue_yaw_2) (`KismetMathLibrary.BreakRotator` (`KismetMathLibrary.RLerp` _returnvalue_3 (`KismetMathLibrary.FindLookAtRotation` _returnvalue (+ _returnvalue (* _returnvalue_4 -1.0))) _lookatalpha true)))
  (if (>= (`KismetMathLibrary.Dot_VectorVector` (`KismetMathLibrary.GetForwardVector` _returnvalue_3) _returnvalue_4) 0.0)
    (`SceneComponent.K2_SetWorldRotation` (`self.Plane`) (`KismetMathLibrary.MakeRotator` _relativerotation_roll _relativerotation_pitch (+ _returnvalue_yaw -90.0)) false false)
    (else
      (`SceneComponent.K2_SetWorldRotation` (`self.Plane`) (`KismetMathLibrary.MakeRotator` _relativerotation_roll _relativerotation_pitch (+ _returnvalue_yaw_2 -90.0)) false false))))

(fn `UserConstructionScript`)