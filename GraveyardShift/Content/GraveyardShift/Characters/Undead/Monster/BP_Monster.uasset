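; BP_Monster is an undead monster character that rises up out of the ground when it spawns.
; BeginPlay teleports it a fixed distance below its placed location, then Tick lerps it back up over RiseDuration without sweeping.
; When the rise completes, it enables capsule collision, restores gravity, and spawns a BP_MonsterController to possess itself, so the controller only takes over once it has surfaced.
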(event `self.ReceiveBeginPlay`
  (bind _returnvalue (`self.K2_GetActorLocation`))
  (set `self.TargetLocation` _returnvalue)
  (bind _output_get (set `self.SpawnedLocation` (- _returnvalue (* (`self.GetActorUpVector`) 600.0))))
  (`self.K2_SetActorLocation` _output_get false true)
  (set `self.bIsRising` true))

(event `self.ReceiveTick`
  (params (DeltaSeconds :type "Float (single-precision)"))
  (bind _returnvalue (`KismetMathLibrary.FClamp` (/ (`self.RiseElapsedTime`) (`self.RiseDuration`))))
  (if (`self.bIsRising`)
    (set `self.RiseElapsedTime` (+ DeltaSeconds (`self.RiseElapsedTime`)))
    (`self.K2_SetActorLocation` (`KismetMathLibrary.VLerp` (`self.SpawnedLocation`) (`self.TargetLocation`) _returnvalue))
    (if (== _returnvalue 1.0)
      (set `self.bIsRising` false)
      (`PrimitiveComponent.SetCollisionEnabled` (`self.CapsuleComponent`) "QueryAndPhysics")
      (set `CharacterMovementComponent.GravityScale` 1.0 (`self.CharacterMovement`))
      (bind _returnvalue_2 (`|SpawnActorFromClass` "/Game/GraveyardShift/Characters/Undead/Monster/BP_MonsterController.BP_MonsterController_C" (`KismetMathLibrary.MakeTransform` (0.0 0.0 0.0)) "Undefined" "MultiplyWithRoot" null null))
      (`Controller.Possess` _returnvalue_2 self))))

(fn `UserConstructionScript`)