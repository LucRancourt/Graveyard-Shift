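; Undead character that rises out of its assigned Grave and can be sent back and buried, triggering the player's win.
; A timeline lifts it from below ground, then enables collision and gravity and spawns a BP_UndeadController to possess it.
; Bury reverses that timeline before destroying the actor, while Freeze and ReturnToGrave drive the AI controller.
; Each tick, its sprite plane yaws between actor facing and the camera axis, flipping by viewing side.
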(event `Bury`
  (`/Engine/EditorBlueprintResources/StandardMacros.Gate` false :!label _label
    (:`Exit`
      (`|ExecutionSequence`
        (:`then_0`
          (goto _label :!via `Close`))
        (:`then_1`
          (`GameplayStatics.PlaySoundAtLocation` (`self.RisingSurfaceSFX`) (`self.K2_GetActorLocation`) (struct) 1.0 1.0 0.0 null null null null)
          ; Rising
          (bind (_direction _rising_floattrack) (`Timeline|Rising_Timeline` :!via `ReverseFromEnd` :!label _label_2)
            (:`Update`
              (`self.RisingMovement` _rising_floattrack)
              (switch `ETimelineDirection` _direction
                (:`Forward`
                  (`/Engine/EditorBlueprintResources/StandardMacros.Gate` false :!label _label_3
                    (:`Exit`
                      (if (>= _rising_floattrack 0.8)
                        (`GameplayStatics.PlaySoundAtLocation` (`self.RisingSurfaceSFX`) (`self.K2_GetActorLocation`) (struct) 1.0 1.0 0.0 null null null null)
                        (goto _label_3 :!via `Close`)))))))
            (:`Finished`
              (switch `ETimelineDirection` _direction
                (:`Forward`
                  (`self.SetupUndeadForController`))
                (:`Backward`
                  (`self.K2_DestroyActor`)
                  (bind _asbp_player_character (cast `/Game/GraveyardShift/Core/Player/BP_PlayerCharacter` (`Controller.K2_GetPawn` (`GameplayStatics.GetPlayerController` 0))))
                  (`/Game/GraveyardShift/Core/Player/BP_PlayerCharacter.PlayerWin` _asbp_player_character))))))))))

(event `self.ReceiveBeginPlay`
  (bind _returnvalue (+ (`self.K2_GetActorLocation` (`self.Grave`)) (0.0 0.0 120.0)))
  (bind _isvalid (`self.IsValidUndead`))
  (if _isvalid
    ; Set StartingPosition Values
    (set `self.TargetLocation` _returnvalue)
    (bind _output_get (set `self.SpawnedLocation` (- _returnvalue (* (`self.GetActorUpVector`) 600.0))))
    (`self.K2_SetActorLocation` _output_get false true)
    ; Rising
    (`TimelineComponent.SetPlayRate` (`self.Rising_Timeline`) (`KismetMathLibrary.SafeDivide` 1.0 (`self.RiseDuration`)))
    (goto _label_2 :!via `PlayFromStart`)))

(event `self.ReceiveTick`
  (params (DeltaSeconds :type "Float (single-precision)"))
  (`self.SpriteLookAt`))

(event `Freeze`
  (`Controller.StopMovement` (`AIBlueprintHelperLibrary.GetAIController` self)))

(event `ReturnToGrave`
  (bind _asbp_undead_controller (cast `/Game/GraveyardShift/Characters/Undead/BP_UndeadController` (`AIBlueprintHelperLibrary.GetAIController` self)))
  (set `self.ExitTarget` (`self.Grave`))
  (`/Game/GraveyardShift/Characters/Undead/BP_UndeadController.SetExitTarget` _asbp_undead_controller))

(fn `IsValidUndead`
  (returns (IsValid :type Boolean))
  (`/Engine/EditorBlueprintResources/StandardMacros.IsValid` (`self.Grave`)
    (:`Is Valid`
      (return true))
    (:`Is Not Valid`
      (`KismetSystemLibrary.PrintString` (`KismetStringLibrary.Concat_StrStr` "ERROR - Grave is NULL on : " (`KismetSystemLibrary.GetDisplayName` self)))
      (return false))))

(fn `RisingMovement`
  (params (InputPin :type "Float (single-precision)"))
  (`self.K2_SetActorLocation` (`KismetMathLibrary.VLerp` (`self.SpawnedLocation`) (`self.TargetLocation`) InputPin)))

(fn `SetupUndeadForController`
  (`|ExecutionSequence`
    (:`then_0`
      ; Character/Capsule
      (`PrimitiveComponent.SetCollisionEnabled` (`self.CapsuleComponent`) "QueryAndPhysics")
      (set `CharacterMovementComponent.GravityScale` 1.0 (`self.CharacterMovement`)))
    (:`then_1`
      ; AI Controller
      (bind _returnvalue (`|SpawnActorFromClass` "/Game/GraveyardShift/Characters/Undead/BP_UndeadController.BP_UndeadController_C" (`KismetMathLibrary.MakeTransform` (0.0 0.0 0.0)) "Undefined" "MultiplyWithRoot" null null))
      (`Controller.Possess` _returnvalue self))))

(fn `SpriteLookAt`
  (bind _returnvalue (`self.K2_GetActorLocation`))
  (bind _returnvalue_2 (`self.K2_GetActorLocation`))
  (bind _lookatalpha (`self.LookAtAlpha`))
  (bind (_relativerotation_roll _relativerotation_pitch) (`KismetMathLibrary.BreakRotator` (`SceneComponent.RelativeRotation` (`self.Plane`))))
  (bind _returnvalue_3 (`KismetMathLibrary.FindLookAtRotation` _returnvalue_2 (+ _returnvalue_2 (`self.GetActorForwardVector`))))
  (bind _returnvalue_4 (`KismetMathLibrary.Normal` (- (`PlayerCameraManager.GetCameraLocation` (`GameplayStatics.GetPlayerCameraManager` 0)) _returnvalue_2)))
  (bind (_returnvalue_roll _returnvalue_pitch _returnvalue_yaw) (`KismetMathLibrary.BreakRotator` (`KismetMathLibrary.RLerp` _returnvalue_3 (`KismetMathLibrary.FindLookAtRotation` _returnvalue (+ _returnvalue _returnvalue_4)) _lookatalpha true)))
  (bind (_returnvalue_roll_2 _returnvalue_pitch_2 _returnvalue_yaw_2) (`KismetMathLibrary.BreakRotator` (`KismetMathLibrary.RLerp` _returnvalue_3 (`KismetMathLibrary.FindLookAtRotation` _returnvalue (+ _returnvalue (* _returnvalue_4 -1.0))) _lookatalpha true)))
  (if (>= (`KismetMathLibrary.Dot_VectorVector` (`KismetMathLibrary.GetForwardVector` _returnvalue_3) _returnvalue_4) 0.0)
    (`SceneComponent.K2_SetWorldRotation` (`self.Plane`) (`KismetMathLibrary.MakeRotator` _relativerotation_roll _relativerotation_pitch (+ _returnvalue_yaw -90.0)) false false)
    (else
      (`SceneComponent.K2_SetWorldRotation` (`self.Plane`) (`KismetMathLibrary.MakeRotator` _relativerotation_roll _relativerotation_pitch (+ _returnvalue_yaw_2 -90.0)) false false))))

(fn `UserConstructionScript`)