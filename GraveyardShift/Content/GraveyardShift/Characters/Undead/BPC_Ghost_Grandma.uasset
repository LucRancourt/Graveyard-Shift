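; Grandma ghost character that targets the player on possession and knocks them back on a cooldown while they overlap its hit volume, calling Freeze when the player is frozen.
; It is satisfied in two stages: dentures first, then a hamburger, which retargets it, disables interaction and reports completion to the ghost counter.
; Material swaps show each stage, with a timed two-material flip animating chewing.
; An item-drop routine remains unconnected.
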(event `self.ReceiveBeginPlay`
  (`parent.ReceiveBeginPlay`)
  (bind _returnvalue (`GameplayStatics.GetActorOfClass` "/Game/GraveyardShift/Core/Player/BP_PlayerCharacter.BP_PlayerCharacter_C"))
  (set `self.PlayerRef` _returnvalue))

(event `self.ReceiveTick`
  (params (DeltaSeconds :type "Float (single-precision)"))
  (bind _player (`self.Player`))
  (`parent.ReceiveTick` DeltaSeconds)
  (`self.GrandmaEatingAnim` DeltaSeconds)
  (if (`/Game/GraveyardShift/Core/Player/BP_PlayerCharacter.IsFrozen` (`self.PlayerRef`))
    (`self.Freeze`)
    (else
      (set `self.CurrentDelayTime` (- (`self.CurrentDelayTime`) DeltaSeconds))
      (`/Engine/EditorBlueprintResources/StandardMacros.IsValid` (`self.Player`)
        (:`Is Valid`
          (if (<= (`self.CurrentDelayTime`) 0.0)
            (`GameplayStatics.PlaySoundAtLocation` (`self.BumpSFX`) (`self.K2_GetActorLocation`) (struct) 1.0 1.0 0.0 null null null null)
            (`self.LaunchCharacter` _player (+ (* (`KismetMathLibrary.Normal` (- (`self.K2_GetActorLocation` _player) (`self.K2_GetActorLocation`))) (`self.GrandmaKnockbackStrength`)) (* (`KismetMathLibrary.Vector_Up`) (`self.GrandmaKnockbackLift`))) false false)
            (set `self.CurrentDelayTime` (`self.DelayBetweenAttacks`))))))))

(event `self.OnItemSuccessBehavior`
  (set `self.HasDentures` true)
  (`PrimitiveComponent.SetMaterial` (`self.Plane`) 0 (`self.GrandmaHasTeethMat`))
  (`GameplayStatics.PlaySoundAtLocation` (`self.GrandmaHungrySFX`) (`self.K2_GetActorLocation`) (struct) 1.0 1.0 0.0 null null null null))

(event `self.GrandmaFearedObjectSuccessBehavior`
  (if (`self.HasDentures`)
    (`PrimitiveComponent.SetMaterial` (`self.Plane`) 0 (`self.GrandmaHasFoodMat_01`))
    (set `self.HasHamburger` true)
    (`self.SetNewTarget` null)
    (`/Game/GraveyardShift/Core/Interactable/BPAC_GhostInteract.DisableInteractableComp` (`self.BPAC_GhostInteract`))
    ; Comment
    (set `self.DesiredObject` "NewEnumerator6")
    (`/Game/GraveyardShift/Core/BP_GhostCounter.CompletedGhost` (`self.GhostCounterRef`))
    (`GameplayStatics.PlaySoundAtLocation` (`self.GrandmaChewing`) (`self.K2_GetActorLocation`) (struct) 1.0 1.0 0.0 null null null null)
    (else
      (`GameplayStatics.PlaySoundAtLocation` (`self.GrandmaTeethSFX`) (`self.K2_GetActorLocation`) (struct) 1.0 1.0 0.0 null null null null))))

(event `self.HitDetection.OnComponentBeginOverlap`
  (params (OverlappedComponent :type "PrimitiveComponent Object Reference") (OtherActor :type "Actor Object Reference") (OtherComp :type "PrimitiveComponent Object Reference") (OtherBodyIndex :type Integer) (bFromSweep :type Boolean) (SweepResult :type "HitResult Structure (by ref)"))
  (bind _asbp_player_character (cast `/Game/GraveyardShift/Core/Player/BP_PlayerCharacter` OtherActor))
  (set `self.Player` _asbp_player_character))

(event `self.HitDetection.OnComponentEndOverlap`
  (params (OverlappedComponent :type "PrimitiveComponent Object Reference") (OtherActor :type "Actor Object Reference") (OtherComp :type "PrimitiveComponent Object Reference") (OtherBodyIndex :type Integer))
  (cast `/Game/GraveyardShift/Core/Player/BP_PlayerCharacter` OtherActor)
  (set `self.Player` null))

(fn `GrandmaEatingAnim`
  (params (Delta :type "Float (double-precision)"))
  (bind _plane (`self.Plane`))
  (if (and (`self.HasDentures`) (`self.HasHamburger`))
    (bind _output_get (set `self.GrandmaEatingSwitchRemaining` (- (`self.GrandmaEatingSwitchRemaining`) Delta)))
    (if (<= _output_get 0.0)
      (set `self.GrandmaEatingSwitchRemaining` (`self.GrandmaEatingSwitchTimer`))
      (if (== (`PrimitiveComponent.GetMaterial` (`self.Plane`) 0) (`self.GrandmaHasFoodMat_01`))
        (`PrimitiveComponent.SetMaterial` _plane 0 (`self.GrandmaHasFoodMat_02`))
        (else
          (`PrimitiveComponent.SetMaterial` _plane 0 (`self.GrandmaHasFoodMat_01`)))))))

(fn `OnPossessed`
  (`parent.OnPossessed`)
  (`self.SetNewTarget` (`self.PlayerRef`)))

(fn `UserConstructionScript`
  (`parent.UserConstructionScript`))