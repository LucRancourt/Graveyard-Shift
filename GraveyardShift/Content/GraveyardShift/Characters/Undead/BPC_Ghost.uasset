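; BPC_Ghost is the ghost undead character in Graveyard Shift, a child Blueprint with a ghost interaction component.
; Its SetEnableInteract event switches that component on or off when it is valid.
; IsValidUndead extends the parent check for instances of exactly this class, printing errors and failing when DesiredObject is left at its null value or ExitTarget is missing.
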(event `SetEnableInteract`
  (params (IsEnabled :type Boolean :default true))
  (bind _bpac_ghostinteract (`self.BPAC_GhostInteract`))
  (`/Engine/EditorBlueprintResources/StandardMacros.IsValid` _bpac_ghostinteract
    (:`Is Valid`
      (`InteractableComponent.SetIsEnabled` _bpac_ghostinteract IsEnabled))))

(fn `IsValidUndead`
  (returns (IsValid :type Boolean))
  (locals (IsValidGhost :type Boolean :default true))
  (bind _returnvalue (`KismetSystemLibrary.GetDisplayName` self))
  (bind _isvalid (`parent.IsValidUndead`))
  (set `local.IsValidGhost` _isvalid)
  (if (== "BPC_Ghost_C" (`GameplayStatics.GetObjectClass` self))
    (if (not (`|EnumInequality` "NewEnumerator1" (`self.DesiredObject`)))
      (`KismetSystemLibrary.PrintString` (`KismetStringLibrary.Concat_StrStr` "ERROR - EnumObject is NULL on : " _returnvalue) true true (struct :`R` 1.0 :`G` 0.015365 :`A` 1.0) 20.0)
      (set `local.IsValidGhost` false))
    (`/Engine/EditorBlueprintResources/StandardMacros.IsValid` (`self.ExitTarget`)
      (:`Is Valid`
        _)
      (:`Is Not Valid`
        (`KismetSystemLibrary.PrintString` (`KismetStringLibrary.Concat_StrStr` "ERROR - ExitTarget is NULL on : " _returnvalue) true true (struct :`R` 1.0 :`G` 0.015209 :`A` 1.0) 20.0)
        (set `local.IsValidGhost` false)))
    (return (`local.IsValidGhost`))))

(fn `UserConstructionScript`
  (`parent.UserConstructionScript`))