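; Drunk ghost character for Graveyard Shift, extending a parent ghost class with its own reactions to item success and end of game.
; On item success it sets a new target, disables its interact component and reports completion to the ghost counter.
; It repositions its Plane component downward if the ghost count is above zero.
; At end of game it resets the Plane's transform with a new rotation, then runs the parent's return-to-grave logic.
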(event `self.OnItemSuccessBehavior`
  (bind _ghostcounterref (`self.GhostCounterRef`))
  (`parent.OnItemSuccessBehavior`)
  (`self.SetNewTarget` null)
  (`/Game/GraveyardShift/Core/Interactable/BPAC_GhostInteract.DisableInteractableComp` (`self.BPAC_GhostInteract`))
  (`/Game/GraveyardShift/Core/BP_GhostCounter.CompletedGhost` _ghostcounterref)
  (if (> (`/Game/GraveyardShift/Core/BP_GhostCounter.GhostCount` _ghostcounterref) 0)
    (`SceneComponent.K2_SetRelativeLocationAndRotation` :`self` (`self.Plane`) :`NewLocation` (0.0 0.0 -70.0))))

(event `self.EndGame_ReturnToGrave`
  (`SceneComponent.K2_SetRelativeLocationAndRotation` (`self.Plane`) (0.0 0.0 0.0) (struct :`Yaw` -90.0 :`Roll` 90.0) false false)
  (`parent.EndGame_ReturnToGrave`))

(fn `UserConstructionScript`
  (`parent.UserConstructionScript`))