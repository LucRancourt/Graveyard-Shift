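; AI controller for undead monsters that runs BT_Undead and feeds it exit, speed, repellent and bait data through the Blackboard.
; On possess, after a short delay, it sets the default monster nav filter, seeds the Blackboard and enables sight.
; Perception updates track repellents and baits in range, targeting the nearest bait and resetting the exit target when a repellent is lost.
; A helper sums normalized directions away from repellents into a flee direction.
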(event `self.ReceivePossess`
  (params (PossessedPawn :type "Pawn Object Reference"))
  (`KismetSystemLibrary.Delay` 0.2)
  (bind _asbp_undead (cast `/Game/GraveyardShift/Characters/Undead/BP_Undead` PossessedPawn))
  (bind _output_get (set `self.Undead` _asbp_undead))
  (`|ExecutionSequence`
    (:`then_0`
      (set `self.DefaultNavigationFilterClass` "/Game/GraveyardShift/Core/AI_Navigation/NavFilter_MonsterDefault.NavFilter_MonsterDefault_C"))
    (:`then_1`
      (`self.RunBehaviorTree` "/Game/GraveyardShift/Characters/Undead/BT_Undead.BT_Undead")
      (`self.SetupBlackboardVariables`)
      (`AIPerceptionComponent.SetSenseEnabled` (`self.AIPerception`) "/Script/AIModule.AISense_Sight" true))))

(event `self.AIPerception.OnTargetPerceptionUpdated`
  (params (Actor :type "Actor Object Reference") (Stimulus :type "AIStimulus Structure"))
  (bind _repellantsinrange (`self.RepellantsInRange`))
  (bind _baitsinrange (`self.BaitsInRange`))
  (bind _inrepellentrange (`self.InRepellentRange`))
  (bind _inbaitrange (`self.InBaitRange`))
  (bind _baitsinrange_2 (`self.BaitsInRange`))
  (bind _closestbaitindex (`self.ClosestBaitIndex`))
  (bind _returnvalue (> (`KismetArrayLibrary.Array_Length` _baitsinrange) 0))
  ; Repellant detection ~ detects any pickup for now
  (bind _asbp_repellent (cast `/Game/GraveyardShift/Core/AI_Navigation/BP_Repellent` Actor)
    (:`then`
      (if Stimulus_bSuccessfullySensed
        (`KismetArrayLibrary.Array_AddUnique` (`self.RepellantsInRange`) _asbp_repellent)
        (`BlackboardComponent.SetValueAsBool` (`self.Blackboard`) _inrepellentrange true)
        (else
          (`KismetArrayLibrary.Array_RemoveItem` _repellantsinrange _asbp_repellent)
          (`BlackboardComponent.SetValueAsBool` (`self.Blackboard`) _inrepellentrange (> (`KismetArrayLibrary.Array_Length` _repellantsinrange) 0))
          (`self.SetExitTarget`))))
    (:`CastFailed`
      (bind _asbp_bait (cast `/Game/GraveyardShift/Core/AI_Navigation/BP_Bait` Actor))
      (if Stimulus_bSuccessfullySensed
        (`KismetArrayLibrary.Array_AddUnique` _baitsinrange _asbp_bait)
        (`BlackboardComponent.SetValueAsBool` (`self.Blackboard`) _inbaitrange true)
        (set `self.ClosestBaitDistance` 100000000000.0 :!label _label)
        (for (_array_element _array_index) _baitsinrange
          (bind _returnvalue_2 (`self.GetDistanceTo` _array_element (`self.GetOwner`)))
          (if (< _returnvalue_2 (`self.ClosestBaitDistance`))
            (set `self.ClosestBaitDistance` _returnvalue_2)
            (set `self.ClosestBaitIndex` _array_index)))
        (if (`KismetArrayLibrary.Array_IsValidIndex` _baitsinrange_2 _closestbaitindex)
          (`BlackboardComponent.SetValueAsObject` (`self.Blackboard`) (`self.TargetBait`) (`|GetArrayItem` _baitsinrange_2 _closestbaitindex)))
        (else
          (`KismetArrayLibrary.Array_RemoveItem` _baitsinrange _asbp_bait)
          (`BlackboardComponent.SetValueAsBool` (`self.Blackboard`) _inbaitrange _returnvalue)
          (if _returnvalue
            (goto _label)))))))

(fn `CalculateRepelledRunDirection`
  (returns (RunDirection :type "Vector Structure"))
  (locals (UndeadPawn :type "Pawn Object Reference") (RunDir :type "Vector Structure" :default (0.0 0.0 0.0)))
  (set `local.UndeadPawn` (`self.K2_GetPawn`))
  (for _array_element (`self.RepellantsInRange`)
    (set `local.RunDir` (+ (`local.RunDir`) (`KismetMathLibrary.Vector_Normal2D` (- (`self.K2_GetActorLocation` (`local.UndeadPawn`)) (`self.K2_GetActorLocation` _array_element))))))
  (return (`KismetMathLibrary.Normal` (`local.RunDir`))))

(fn `SetExitTarget`
  (`BlackboardComponent.SetValueAsObject` (`self.Blackboard`) (`self.TargetExit`) (`/Game/GraveyardShift/Characters/Undead/BP_Undead.ExitTarget` (`self.Undead`))))

(fn `SetSpeeds`
  (`|ExecutionSequence`
    (:`then_0`
      (`BlackboardComponent.SetValueAsFloat` (`self.Blackboard`) (`self.WalkSpeed`) (`/Game/GraveyardShift/Characters/Undead/BP_Undead.WalkSpeed` (`self.Undead`))))
    (:`then_1`
      (`BlackboardComponent.SetValueAsFloat` (`self.Blackboard`) (`self.RunAwaySpeed`) (`/Game/GraveyardShift/Characters/Undead/BP_Undead.RunAwaySpeed` (`self.Undead`))))
    (:`then_2`
      (`BlackboardComponent.SetValueAsFloat` (`self.Blackboard`) (`self.ChaseSpeed`) (`/Game/GraveyardShift/Characters/Undead/BP_Undead.ChaseSpeed` (`self.Undead`))))))

(fn `SetupBlackboardVariables`
  (`self.SetExitTarget`)
  (`self.SetSpeeds`))

(fn `UserConstructionScript`)