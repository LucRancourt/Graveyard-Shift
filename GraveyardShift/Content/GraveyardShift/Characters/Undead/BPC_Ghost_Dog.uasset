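; Ghost dog undead character that roams between pickups, carries them in its mouth and chases the player to steal held items.
; Tick drives speed and state, starting a chase when the player's hold timer expires; catching the player freezes them, turns their view and takes the item.
; A repeating timer drops and retargets to random pickups.
; Its desired item makes it chew, temporarily counting as completed until the distraction ends.
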(event `self.ReceiveBeginPlay`
  (bind _allpickups (`self.AllPickups`))
  (`parent.ReceiveBeginPlay`)
  (bind _returnvalue (`GameplayStatics.GetActorOfClass` "/Game/GraveyardShift/Core/Player/BP_PlayerCharacter.BP_PlayerCharacter_C"))
  (bind _output_get (set `self.PlayerRef` _returnvalue))
  (add `/Game/GraveyardShift/Core/Player/BP_PlayerCharacter.OnPickup` _output_get (delegate `OnPickup_Event`))
  (add `/Game/GraveyardShift/Core/Player/BP_PlayerCharacter.OnDrop` _output_get (delegate `OnDrop_Event`))
  (bind _outactors (`GameplayStatics.GetAllActorsOfClass` "/Game/GraveyardShift/Core/Interactable/BP_Pickup.BP_Pickup_C"))
  (bind _output_get_2 (set `self.AllPickups` _outactors))
  (if (not (`self.CanPickupBone`))
    (for _array_element _allpickups
      (if (`|EnumEquality` (`/Game/GraveyardShift/Core/Interactable/BP_Pickup.DesiredObjectIdentifier` _array_element) "NewEnumerator2")
        (`KismetArrayLibrary.Array_RemoveItem` _allpickups _array_element)
        (break))))
  (for _array_element_2 (`self.AllPickups`)
    (bind _returnvalue_2 (`KismetMathLibrary.Vector_Distance` (`self.K2_GetActorLocation`) (`self.K2_GetActorLocation` _array_element_2)))
    (if (< _returnvalue_2 (`self.ShortestDistanceFor1stTarget`))
      (set `self.TempTarget` _array_element_2)
      (set `self.ShortestDistanceFor1stTarget` _returnvalue_2)))
  (`/Engine/EditorBlueprintResources/StandardMacros.IsValid` (`self.TempTarget`)
    (:`Is Valid`
      (set `self.ChaseSpeed` (`self.WalkSpeed`)))
    (:`Is Not Valid`
      (`KismetSystemLibrary.PrintString` "ERROR ON DOG BEGINPLAY"))))

(event `OnPickup_Event`
  (bind _playerref (`self.PlayerRef`))
  (set `self.PlayerHeldItem` (`/Game/GraveyardShift/Core/Player/BP_PlayerCharacter.HeldItemEnum` _playerref))
  (if (!= (`self.Target`) (`/Game/GraveyardShift/Core/Player/BP_PlayerCharacter.HeldPickup` _playerref))
    (set `self.PlayerHoldItemTimeRemaining` (`self.PlayerHoldItemTime`))))

(event `OnDrop_Event`
  (set `self.PlayerHeldItem` 99))

(event `self.ReceiveTick`
  (params (DeltaSeconds :type "Float (single-precision)"))
  (bind _playerref (`self.PlayerRef`))
  (bind _temptarget (`self.TempTarget`))
  (bind _helditem (`self.HeldItem`))
  (bind _bpac_ghostinteract (`self.BPAC_GhostInteract`))
  (bind _walkspeed (`self.WalkSpeed`))
  (bind _dogchasespeed (`self.DogChaseSpeed`))
  (bind _target (`self.Target`))
  (bind _held_pickup (`/Game/GraveyardShift/Core/Interactable/BPAC_GhostInteract.Held Pickup` _bpac_ghostinteract))
  (bind _heldpickup (`/Game/GraveyardShift/Core/Player/BP_PlayerCharacter.HeldPickup` _playerref))
  (`/Engine/EditorBlueprintResources/StandardMacros.IsValid` (`AIBlueprintHelperLibrary.GetAIController` self)
    (:`Is Valid`
      (`parent.ReceiveTick` DeltaSeconds)
      (if (`/Game/GraveyardShift/Core/Player/BP_PlayerCharacter.IsFrozen` (`self.PlayerRef`))
        (`self.UpdateSpeeds` 0.0)
        (else
          (if (or (== _walkspeed _dogchasespeed) (== _walkspeed 0.0))
            (if (`self.IsChasing`)
              (`self.UpdateSpeeds` _dogchasespeed)
              (else
                (`self.UpdateSpeeds` (`self.ChaseSpeed`)))))
          (if (`self.IsActive`)
            (if (and (`KismetSystemLibrary.IsValid` _target) (and (not (`self.IsChasing`)) (== _target (`/Game/GraveyardShift/Core/Player/BP_PlayerCharacter.HeldPickup` (`self.PlayerRef`)))))
              (`self.SetNewPickupTarget`))
            (if (!= (`self.PlayerHeldItem`) 99)
              (if (== (`self.PlayerHeldItem`) (`/Game/GraveyardShift/Core/Player/BP_PlayerCharacter.HeldItemEnum` (`self.PlayerRef`)))
                (bind _output_get (set `self.PlayerHoldItemTimeRemaining` (- (`self.PlayerHoldItemTimeRemaining`) DeltaSeconds)))
                (if (<= _output_get 0.0) :!label _label
                  (set `self.IsChasing` true)
                  (`/Engine/EditorBlueprintResources/StandardMacros.IsValid` (`self.HeldItem`)
                    (:`Is Valid`
                      (`self.DogDropPickup`))
                    (:`Is Not Valid`
                      _))
                  (`/Engine/EditorBlueprintResources/StandardMacros.IsValid` _heldpickup
                    (:`Is Valid`
                      (set `self.TempTarget` _heldpickup)
                      (if (!= (`self.Target`) _playerref)
                        (`self.SetNewTarget` (`self.PlayerRef`))
                        (`self.UpdateSpeeds` (`self.DogChaseSpeed`) :!label _label_2)))
                    (:`Is Not Valid`
                      ; Did Player just Drop the Item to prevent the Dog's Chase?
                      (if (== (`self.PlayerHeldItem`) 99)
                        (if (!= _temptarget (`self.Target`))
                          (`self.SetNewTarget` _temptarget)
                          (goto _label_2)))))))
              (else
                (goto _label)))
            (elif (== (`self.Target`) (`self.Grave`))
              (`self.UpdateSpeeds` 800.0)
              (else
                (bind _output_get_2 (set `self.BoneDistractionDurationRemaining` (- (`self.BoneDistractionDurationRemaining`) DeltaSeconds)))
                (set `self.IsChasing` false)
                (`self.UpdateSpeeds` 0.0)
                (`self.SetNewTarget` null)
                (if (<= _output_get_2 0.0)
                  (if (not (== (`self.Target`) (`self.Grave`)))
                    (`/Game/GraveyardShift/Core/Interactable/BPAC_GhostInteract.EnableInteractableComp` (`self.BPAC_GhostInteract`))
                    (`self.SetMat` false)
                    (`/Game/GraveyardShift/Core/BP_GhostCounter.AddGhost` (`self.GhostCounterRef`))
                    (`/Engine/EditorBlueprintResources/StandardMacros.IsValid` _held_pickup
                      (:`Is Valid`
                        (`SceneComponent.SetHiddenInGame` (`/Game/GraveyardShift/Core/Interactable/BP_Pickup.Sprite` _held_pickup) false true)
                        (`/Game/GraveyardShift/Core/Interactable/BP_Pickup.Drop` _held_pickup)
                        (set `/Game/GraveyardShift/Core/Interactable/BPAC_GhostInteract.Held Pickup` null _bpac_ghostinteract))
                      (:`Is Not Valid`
                        (`/Engine/EditorBlueprintResources/StandardMacros.IsValid` _helditem
                          (:`Is Valid`
                            (`self.SetActorHiddenInGame` _helditem false)
                            (`self.DogDropPickup`)))))
                    (set `self.IsActive` true)
                    (`self.UpdateSpeeds` (`self.ChaseSpeed`))
                    (`self.SetNewPickupTarget`)))))))))))

(event `self.OnItemSuccessBehavior`
  (bind _helditem (`self.HeldItem`))
  (`parent.OnItemSuccessBehavior` :!label _label_3)
  (`GameplayStatics.PlaySoundAtLocation` (`self.DogChewing`) (`self.K2_GetActorLocation`) (struct) 1.0 1.0 0.0 null null null null)
  (set `self.BoneDistractionDurationRemaining` (`self.BoneDistractionDuration`))
  (`/Game/GraveyardShift/Core/Interactable/BPAC_GhostInteract.DisableInteractableComp` (`self.BPAC_GhostInteract`))
  (`/Engine/EditorBlueprintResources/StandardMacros.IsValid` _helditem
    (:`Is Valid`
      (if (`|EnumEquality` (`/Game/GraveyardShift/Core/Interactable/BP_Pickup.DesiredObjectIdentifier` _helditem) (`self.DesiredObject`))
        (`self.SetActorHiddenInGame` _helditem true)
        (else
          (`self.DogDropPickup`))))
    (:`Is Not Valid`
      _))
  (set `self.IsActive` false)
  (`/Game/GraveyardShift/Core/BP_GhostCounter.CompletedGhost` (`self.GhostCounterRef`)))

(event `self.HitCollider.OnComponentBeginOverlap`
  (params (OverlappedComponent :type "PrimitiveComponent Object Reference") (OtherActor :type "Actor Object Reference") (OtherComp :type "PrimitiveComponent Object Reference") (OtherBodyIndex :type Integer) (bFromSweep :type Boolean) (SweepResult :type "HitResult Structure (by ref)"))
  (bind _timerhandle (`self.TimerHandle`))
  (bind _timerhandle_2 (`self.TimerHandle`))
  (bind _helditem (`self.HeldItem`))
  (bind _playerref (`self.PlayerRef`))
  (bind _newitemcollided (`self.NewItemCollided`))
  (bind _helditem_2 (`self.HeldItem`))
  (bind _playerref_2 (`self.PlayerRef`))
  (bind _returnvalue (`self.K2_GetActorLocation` (`GameplayStatics.GetPlayerCameraManager` 0)))
  (bind (_returnvalue_roll _returnvalue_pitch _returnvalue_yaw) (`KismetMathLibrary.BreakRotator` (`KismetMathLibrary.FindLookAtRotation` (`self.K2_GetActorLocation`) _returnvalue)))
  (bind _asbp_player_character (cast `/Game/GraveyardShift/Core/Player/BP_PlayerCharacter` OtherActor)
    (:`then`
      (if (`self.IsChasing`)
        (if (== (`self.Target`) _asbp_player_character)
          (set `self.IsChasing` false)
          (`self.UpdateSpeeds` 0.0)
          (if (not (`/Game/GraveyardShift/Core/Player/BP_PlayerCharacter.IsFrozen` _playerref_2))
            (`/Game/GraveyardShift/Core/Player/BP_PlayerCharacter.Freeze` _asbp_player_character 0.2)
            (`/Engine/EditorBlueprintResources/StandardMacros.IsValid` (`/Game/GraveyardShift/Core/Player/BP_PlayerCharacter.HeldPickup` _asbp_player_character)
              (:`Is Valid`
                (`KismetSystemLibrary.Delay` 0.2)
                (`/Game/GraveyardShift/Core/Player/BP_PlayerCharacter.Freeze` _asbp_player_character 2.0)
                (`/Game/GraveyardShift/Core/Player/BP_PlayerCharacter.Freeze` _playerref_2 2.0)
                (`InteracterComponent.TempDisable` (`/Game/GraveyardShift/Core/Player/BP_PlayerCharacter.Interacter` _playerref_2) 5.0)
                (`self.Freeze`)
                (`self.K2_SetActorRotation` (`KismetMathLibrary.MakeRotator` 0.0 0.0 _returnvalue_yaw))
                (`Controller.SetControlRotation` (`GameplayStatics.GetPlayerController` 0) (`KismetMathLibrary.FindLookAtRotation` (`KismetMathLibrary.MakeVector` (.x _returnvalue) (.y _returnvalue) (.z _returnvalue)) (`KismetMathLibrary.MakeVector` (.x (`SceneComponent.K2_GetComponentLocation` (`self.InteractLookAtLocation`))) (.y (`SceneComponent.K2_GetComponentLocation` (`self.InteractLookAtLocation`))) (.z (`SceneComponent.K2_GetComponentLocation` (`self.InteractLookAtLocation`))))))
                (`KismetSystemLibrary.Delay` 1.0)
                (`/Engine/EditorBlueprintResources/StandardMacros.IsValid` (`self.HeldItem`)
                  (:`Is Valid`
                    (`self.DogDropPickup`))
                  (:`Is Not Valid`
                    _))
                (set `self.HeldItem` (`/Game/GraveyardShift/Core/Player/BP_PlayerCharacter.HeldPickup` _playerref))
                (`/Game/GraveyardShift/Core/Player/BP_PlayerCharacter.DropPickup` _playerref)
                (set `self.PlayerHoldItemTimeRemaining` (`self.PlayerHoldItemTime`))
                (`self.UpdateSpeeds` (`self.ChaseSpeed`))
                (`/Engine/EditorBlueprintResources/StandardMacros.IsValid` _helditem_2
                  (:`Is Valid`
                    (if (`|EnumEquality` (`self.DesiredObject`) (`/Game/GraveyardShift/Core/Interactable/BP_Pickup.DesiredObjectIdentifier` _helditem_2))
                      (if (`KismetSystemLibrary.K2_IsValidTimerHandle` _timerhandle)
                        (`KismetSystemLibrary.K2_ClearAndInvalidateTimerHandle` _timerhandle)
                        (goto _label_3)
                        (else
                          (goto _label_3)))
                      (else
                        (`self.DogPickupPickup`))))
                  (:`Is Not Valid`
                    _))
                (`self.SetNewTarget` null :!label _label_4)
                (set `self.IsChasing` false)
                (set `self.IsActive` true)
                (if (`KismetSystemLibrary.K2_IsValidTimerHandle` _timerhandle_2)
                  (if (`KismetSystemLibrary.K2_IsTimerActiveHandle` _timerhandle_2)
                    (`KismetSystemLibrary.K2_ClearAndInvalidateTimerHandle` _timerhandle_2)))
                (bind _returnvalue_2 (`KismetSystemLibrary.K2_SetTimerDelegate` (delegate `NewTargetAfterDelay`) 12.0 :!label _label_5))
                (set `self.TimerHandle` _returnvalue_2)))))))
    (:`CastFailed`
      (`/Engine/EditorBlueprintResources/StandardMacros.IsValid` _newitemcollided
        (:`Is Not Valid`
          (bind _asbp_pickup (cast `/Game/GraveyardShift/Core/Interactable/BP_Pickup` OtherActor))
          (bind _output_get (set `self.NewItemCollided` _asbp_pickup))
          (if (== (`self.PrevHeldItem`) _newitemcollided)
            _
            (elif (`self.IsChasing`)
              (if (== (`self.Target`) _newitemcollided)
                (set `self.IsChasing` false)
                (set `self.PlayerHoldItemTimeRemaining` (`self.PlayerHoldItemTime`))
                (`self.UpdateSpeeds` (`self.ChaseSpeed`))
                (if (!= (`/Game/GraveyardShift/Core/Interactable/BP_Pickup.DesiredObjectIdentifier` _output_get) (`self.PlayerHeldItem`)) :!label _label_6
                  (`/Engine/EditorBlueprintResources/StandardMacros.IsValid` _helditem
                    (:`Is Valid`
                      (if (!= _helditem (`self.NewItemCollided`))
                        (`self.DogDropPickup`)
                        (`KismetSystemLibrary.Delay` 0.2)
                        (set `self.HeldItem` (`self.NewItemCollided`) :!label _label_7)
                        (`self.DogPickupPickup`)))
                    (:`Is Not Valid`
                      (goto _label_7))))
                (else
                  (set `self.NewItemCollided` null :!label _label_8)))
              (else
                (goto _label_6)))))))))

(event `self.HitCollider.OnComponentEndOverlap`
  (params (OverlappedComponent :type "PrimitiveComponent Object Reference") (OtherActor :type "Actor Object Reference") (OtherComp :type "PrimitiveComponent Object Reference") (OtherBodyIndex :type Integer))
  (bind _newitemcollided (`self.NewItemCollided`))
  (`/Engine/EditorBlueprintResources/StandardMacros.IsValid` _newitemcollided
    (:`Is Valid`
      (if (== _newitemcollided OtherActor)
        (goto _label_8)))))

(event `DogDropPickup`
  (bind _helditem (`self.HeldItem`))
  (bind _returnvalue (`self.GetComponentByClass` _helditem "/Game/GraveyardShift/Core/BPAC_FollowDogMouth.BPAC_FollowDogMouth_C"))
  (`/Engine/EditorBlueprintResources/StandardMacros.IsValid` _helditem
    (:`Is Valid`
      (`/Engine/EditorBlueprintResources/StandardMacros.IsValid` _returnvalue
        (:`Is Valid`
          (set `/Game/GraveyardShift/Core/BPAC_FollowDogMouth.FollowPoint` null _returnvalue))
        (:`Is Not Valid`
          _))
      (`/Game/GraveyardShift/Core/Interactable/BP_Pickup.EnablePickup` _helditem)
      (set `self.PrevHeldItem` _helditem)
      (set `self.HeldItem` null))))

(event `DogPickupPickup`
  (bind _helditem (`self.HeldItem`))
  (`/Game/GraveyardShift/Core/Interactable/BP_Pickup.DisablePickup` _helditem)
  (set `self.NewItemCollided` null)
  (set `/Game/GraveyardShift/Core/BPAC_FollowDogMouth.FollowPoint` (`self.HeldItemLocation`) (`self.GetComponentByClass` _helditem "/Game/GraveyardShift/Core/BPAC_FollowDogMouth.BPAC_FollowDogMouth_C"))
  (goto _label_4))

(event `NewTargetAfterDelay`
  (if (and (`self.IsActive`) (not (`self.IsChasing`)))
    (bind _successfullyfoundpickuptarget (`self.SetNewPickupTarget`))
    (`self.DogDropPickup`)
    (set `self.NewItemCollided` (`self.HeldItem`))
    (if (not _successfullyfoundpickuptarget)
      (goto _label_5))))

(event `RefreshPickupList`
  (bind _allpickups (`self.AllPickups`))
  (bind _target (`self.Target`))
  (bind _asbp_pickup (cast `/Game/GraveyardShift/Core/Interactable/BP_Pickup` _target)
    (:`then`
      (if (== (`KismetArrayLibrary.Array_Find` _allpickups _asbp_pickup) -1)
        (`self.SetNewPickupTarget` :!label _label_9)))
    (:`CastFailed`
      (bind _asbp_player_character (cast `/Game/GraveyardShift/Core/Player/BP_PlayerCharacter` _target))
      (bind _heldpickup (`/Game/GraveyardShift/Core/Player/BP_PlayerCharacter.HeldPickup` _asbp_player_character))
      (`/Engine/EditorBlueprintResources/StandardMacros.IsValid` _heldpickup
        (:`Is Valid`
          (if (== (`KismetArrayLibrary.Array_Find` _allpickups _heldpickup) -1)
            (goto _label_9)))))))

(fn `OnPossessed`
  (`parent.OnPossessed`)
  (`self.SetNewTarget` (`self.TempTarget`))
  (bind _asbp_undead_controller (cast `/Game/GraveyardShift/Characters/Undead/BP_UndeadController` (`AIBlueprintHelperLibrary.GetAIController` self)))
  (`/Game/GraveyardShift/Characters/Undead/BP_UndeadController.SetWander` _asbp_undead_controller true)
  (`GameplayStatics.PlaySoundAtLocation` (`self.DogHowl`) (`self.K2_GetActorLocation`) (struct) 1.0 1.0 0.0 null null null null))

(fn `SetNewPickupTarget`
  (returns (SuccessfullyFoundPickupTarget :type Boolean))
  (locals (IsDone :type Boolean) (FoundTargetPickup :type Boolean) (ValidPickupTargets :type "Array of /Game/GraveyardShift/Core/Interactable/BP_Pickup Object Reference"))
  (bind _validpickuptargets (`local.ValidPickupTargets`))
  (bind _temptarget (`self.TempTarget`))
  (bind _returnvalue (`KismetArrayLibrary.Array_Length` (`self.AllPickups`)))
  (set `self.TempTarget` null)
  (if (and (== _returnvalue 2) (and (`KismetSystemLibrary.IsValid` (`/Game/GraveyardShift/Core/Player/BP_PlayerCharacter.HeldPickup` (`self.PlayerRef`))) (`KismetSystemLibrary.IsValid` (`self.HeldItem`))))
    (`self.SetNewTarget` null :!label _label)
    (set `local.FoundTargetPickup` false)
    (elif (>= _returnvalue 1)
      (for _array_element (`self.AllPickups`)
        (if (and (!= (`/Game/GraveyardShift/Core/Player/BP_PlayerCharacter.HeldPickup` (`self.PlayerRef`)) _array_element) (!= (`self.HeldItem`) _array_element))
          (`KismetArrayLibrary.Array_Add` (`local.ValidPickupTargets`) _array_element)))
      (if (!= (`.OutIndex` (`KismetArrayLibrary.Array_Random` _validpickuptargets)) -1)
        (set `self.TempTarget` (`KismetArrayLibrary.Array_Random` _validpickuptargets))
        (set `local.FoundTargetPickup` true)
        (if (<= (`KismetMathLibrary.Vector_Distance` (`self.K2_GetActorLocation`) (`self.K2_GetActorLocation` _temptarget)) 200.0)
          (goto _label)
          (else
            (`self.SetNewTarget` _temptarget)))
        (else
          (goto _label)))
      (else
        (goto _label))))
  (return (`local.FoundTargetPickup`)))

(fn `UserConstructionScript`
  (`parent.UserConstructionScript`))