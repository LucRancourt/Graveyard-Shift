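; Ballerina ghost character that chases detected players and spins them on contact unless they hold her desired item, leaving for a random exit after enough spins.
; Item success sends her to the map center, where she retargets all other ghosts onto herself and spins to music and light.
; When the timed dance ends she returns to her grave and restores the ghosts' saved targets, or sends them to their graves if all are completed.
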(event `self.OnItemSuccessBehavior`
  (`parent.OnItemSuccessBehavior`)
  (`self.UpdateSpeeds` 125.0)
  (`|ExecutionSequence`
    (:`then_0`
      (goto _label_3 :!via `Close`))
    (:`then_1`
      (`/Game/GraveyardShift/Core/Interactable/BPAC_GhostInteract.DisableInteractableComp` (`self.BPAC_GhostInteract`))
      (`/Game/GraveyardShift/Characters/Undead/BP_UndeadController.SetWander` (`self.UController`) false)
      (`self.SetNewTarget` (`self.CenterOfMap`))
      (set `self.NumSpinPlayerBeforeExit` -1)
      (`/Game/GraveyardShift/Core/BP_GhostCounter.CompletedGhost` (`self.GhostCounterRef`)))))

(event `self.PlayerDetectionCollider.OnComponentBeginOverlap`
  (params (OverlappedComponent :type "PrimitiveComponent Object Reference") (OtherActor :type "Actor Object Reference") (OtherComp :type "PrimitiveComponent Object Reference") (OtherBodyIndex :type Integer) (bFromSweep :type Boolean) (SweepResult :type "HitResult Structure (by ref)"))
  (if true
    (if (> (`self.NumSpinPlayerBeforeExit`) 0)
      (bind _asbp_player_character (cast `/Game/GraveyardShift/Core/Player/BP_PlayerCharacter` OtherActor))
      (if (!= _asbp_player_character (`self.Target`))
        (`self.SetNewTarget` _asbp_player_character)
        (`GameplayStatics.PlaySoundAtLocation` "/Game/GraveyardShift/Audio/SFX/Ghost/Ballerina/SFX_Ballerina_DanceWithMe.SFX_Ballerina_DanceWithMe" (`self.K2_GetActorLocation`) (struct) 1.0 1.0 0.0 null null null null)))))

(event `self.ReceiveTick`
  (params (DeltaSeconds :type "Float (single-precision)"))
  (`parent.ReceiveTick` DeltaSeconds)
  (set `self.PlayerSpinCooldownRemaining` (- (`self.PlayerSpinCooldownRemaining`) DeltaSeconds))
  (`/Engine/EditorBlueprintResources/StandardMacros.Gate` true :!label _label
    (:`Exit`
      (if (!= (`self.Target`) (`self.Grave`))
        (`|ExecutionSequence`
          (:`then_0`
            (`/Engine/EditorBlueprintResources/StandardMacros.Gate` true :!label _label_2
              (:`Exit`
                (`GameplayStatics.PlaySoundAtLocation` (`self.DanceMusic`) (`self.K2_GetActorLocation`) (struct) 1.0 1.0 0.0 null null null null)
                (`LightComponent.SetIntensity` (`self.DanceLight`) 500000.0)
                (goto _label_2 :!via `Close`))))
          (:`then_1`
            (`self.K2_AddActorWorldRotation` (`KismetMathLibrary.MakeRotator` 0.0 0.0 (`self.SpinAmount`)))
            (bind _output_get (set `self.HypnoticDanceDuration` (- (`self.HypnoticDanceDuration`) DeltaSeconds)))
            (if (<= _output_get 0.0)
              (`self.ReturnToGrave`)
              (`LightComponent.SetIntensity` (`self.DanceLight`) 0.0)
              (`KismetSystemLibrary.Delay` 0.4)
              (if (`/Game/GraveyardShift/Core/BP_GhostCounter.AllGhostsCompleted` (`self.GhostCounterRef`))
                (for _array_element (`self.GhostRefs`)
                  (`self.SetNewTarget` _array_element (`/Game/GraveyardShift/Characters/Undead/BP_Undead.Grave` _array_element)))
                (`KismetArrayLibrary.Array_Clear` (`self.GhostRefs`))
                (`KismetArrayLibrary.Array_Clear` (`self.GhostTargetRefs`))
                (else
                  (for (_array_element_2 _array_index) (`self.GhostRefs`)
                    (`self.SetNewTarget` _array_element_2 (`|GetArrayItem` (`self.GhostTargetRefs`) _array_index)))
                  (`KismetArrayLibrary.Array_Clear` (`self.GhostRefs`))
                  (`KismetArrayLibrary.Array_Clear` (`self.GhostTargetRefs`)))))))))))

(event `self.CenterCollider.OnComponentBeginOverlap`
  (params (OverlappedComponent :type "PrimitiveComponent Object Reference") (OtherActor :type "Actor Object Reference") (OtherComp :type "PrimitiveComponent Object Reference") (OtherBodyIndex :type Integer) (bFromSweep :type Boolean) (SweepResult :type "HitResult Structure (by ref)"))
  (if (== OtherActor (`self.CenterOfMap`))
    (bind _outactors (`GameplayStatics.GetAllActorsOfClass` "/Game/GraveyardShift/Characters/Undead/BPC_Ghost.BPC_Ghost_C"))
    (for _array_element _outactors
      (if (!= _array_element self)
        (`KismetArrayLibrary.Array_Add` (`self.GhostRefs`) _array_element)
        (`KismetArrayLibrary.Array_Add` (`self.GhostTargetRefs`) (`/Game/GraveyardShift/Characters/Undead/BP_Undead.Target` _array_element))
        (`self.SetNewTarget` _array_element self)))
    (`|ExecutionSequence`
      (:`then_0`
        (goto _label :!via `Open`))
      (:`then_1`
        (goto _label_2 :!via `Open`)))))

(event `self.PlayerHitCollider.OnComponentBeginOverlap`
  (params (OverlappedComponent :type "PrimitiveComponent Object Reference") (OtherActor :type "Actor Object Reference") (OtherComp :type "PrimitiveComponent Object Reference") (OtherBodyIndex :type Integer) (bFromSweep :type Boolean) (SweepResult :type "HitResult Structure (by ref)"))
  (if (> (`self.NumSpinPlayerBeforeExit`) 0)
    (if (<= (`self.PlayerSpinCooldownRemaining`) 0.0)
      (if (`self.HasBeenPossessed`)
        (bind _asbp_player_character (cast `/Game/GraveyardShift/Core/Player/BP_PlayerCharacter` OtherActor))
        (if (not (`/Game/GraveyardShift/Core/Player/BP_PlayerCharacter.IsFrozen` _asbp_player_character))
          (set `self.PlayerSpinCooldownRemaining` (`self.PlayerSpinCooldown`))
          (if (== (`self.DesiredObject`) (`/Game/GraveyardShift/Core/Player/BP_PlayerCharacter.HeldItemEnum` _asbp_player_character))
            (`KismetSystemLibrary.Delay` 3.0)
            (`/Engine/EditorBlueprintResources/StandardMacros.Gate` false :!label _label_3
              (:`Exit`
                (`self.SetNewTarget` null :!label _label_4)
                (`/Game/GraveyardShift/Characters/Undead/BP_UndeadController.SetWander` (`self.UController`) true)))
            (else
              (`/Game/GraveyardShift/Core/Player/BP_PlayerCharacter.Spin` _asbp_player_character)
              (`KismetSystemLibrary.Delay` (`/Game/GraveyardShift/Core/Player/BP_PlayerCharacter.SpinDuration` _asbp_player_character))
              (bind _result (`/Engine/EditorBlueprintResources/StandardMacros.DecrementInt` (`self.NumSpinPlayerBeforeExit`))
                (:`  `
                  (if (<= _result 0)
                    (bind _outactors (`GameplayStatics.GetAllActorsOfClass` "/Game/GraveyardShift/Core/BP_Exit.BP_Exit_C"))
                    (`self.SetNewTarget` (`KismetArrayLibrary.Array_Random` _outactors))
                    (else
                      (goto _label_4))))))))))))

(fn `OnPossessed`
  (bind _asbp_undead_controller (cast `/Game/GraveyardShift/Characters/Undead/BP_UndeadController` (`self.GetController`)))
  (bind _output_get (set `self.UController` _asbp_undead_controller))
  (`/Game/GraveyardShift/Characters/Undead/BP_UndeadController.SetWander` _output_get true)
  (`parent.OnPossessed`))

(fn `UserConstructionScript`
  (`parent.UserConstructionScript`))