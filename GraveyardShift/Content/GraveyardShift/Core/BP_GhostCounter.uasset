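; BP_GhostCounter tracks how many ghosts are left to complete and to bury, and drives the day-night lighting mood.
; On Tick it lowers post-process color temperature from warm back to its base over SecondsUntilNight.
; Completing the last ghost plays a ping, fires AllGhostCompleted and runs a sunlight timeline on that temperature.
; Burying the last fires AllGhostBuried, with a delayed check for no remaining ghost actors as fallback.
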(event `AddGhost`
  (`/Engine/EditorBlueprintResources/StandardMacros.IncrementInt` (`self.GhostCount`)
    (:`  `
      (`/Engine/EditorBlueprintResources/StandardMacros.IncrementInt` (`self.GhostsToBury`)))))

(event `CompletedGhost`
  (bind _result (`/Engine/EditorBlueprintResources/StandardMacros.DecrementInt` (`self.GhostCount`))
    (:`  `
      (if (<= _result 0)
        (`GameplayStatics.PlaySound2D` "/Engine/EngineSounds/1kSineTonePing.1kSineTonePing" 1.0 1.0 0.0 null null)
        (`KismetSystemLibrary.Delay` 0.3)
        (`self.OnAllGhostCompleted`)
        (set `self.AllGhostsCompleted` true)
        (`/Engine/EditorBlueprintResources/StandardMacros.Gate` false :!label _label
          (:`Exit`
            (`/Engine/EditorBlueprintResources/StandardMacros.IsValid` (`self.PostProcessVolume`)
              (:`Is Valid`
                (`|ExecutionSequence`
                  (:`then_0`
                    (goto _label :!via `Close`))
                  (:`then_1`
                    (bind (_direction _track) (`Timeline|Sunlight_Timeline` :`NewTime` 5.0 :!via `PlayFromStart`)
                      (:`Update`
                        (setmembers `PostProcessSettings` :`StructRef` (`PostProcessVolume.Settings` (`self.PostProcessVolume`)) :`WhiteTemp` (+ _track (`self.BaseTemp`)))))))))))))))

(event `GhostBuried`
  (bind _result (`/Engine/EditorBlueprintResources/StandardMacros.DecrementInt` (`self.GhostsToBury`))
    (:`  `
      (if (<= _result 0)
        (`self.OnAllGhostBuried` :!label _label_2)
        (goto _label_3 :!via `Close`)
        (else
          (`KismetSystemLibrary.Delay` 2.0)
          (`/Engine/EditorBlueprintResources/StandardMacros.Gate` false :!label _label_3
            (:`Exit`
              (bind _outactors (`GameplayStatics.GetAllActorsOfClass` "/Game/GraveyardShift/Characters/Undead/BPC_Ghost.BPC_Ghost_C"))
              (if (`KismetArrayLibrary.Array_IsEmpty` _outactors)
                (goto _label_2)))))))))

(event `self.ReceiveTick`
  (params (DeltaSeconds :type "Float (single-precision)"))
  (bind _basetemp (`self.BaseTemp`))
  (bind _secondsuntilnight (`self.SecondsUntilNight`))
  (bind _settings (`PostProcessVolume.Settings` (`self.PostProcessVolume`)))
  (`/Engine/EditorBlueprintResources/StandardMacros.Gate` true :!label _label_4
    (:`Exit`
      (bind _output_get (set `self.NewTime` (+ DeltaSeconds (`self.NewTime`))))
      (if (>= _output_get _secondsuntilnight)
        (setmembers `PostProcessSettings` :`StructRef` _settings :`WhiteTemp` _basetemp)
        (goto _label_4 :!via `Close`)
        (else
          (setmembers `PostProcessSettings` :`StructRef` _settings :`WhiteTemp` (- (+ _basetemp 10000.0) (* (`self.NewTime`) (`KismetMathLibrary.SafeDivide` 10000.0 _secondsuntilnight)))))))))

(event `self.ReceiveBeginPlay`
  (bind _returnvalue (`GameplayStatics.GetActorOfClass` "/Script/Engine.PostProcessVolume"))
  (bind _output_get (set `self.PostProcessVolume` _returnvalue))
  (`/Engine/EditorBlueprintResources/StandardMacros.IsValid` _output_get
    (:`Is Valid`
      (set `self.BaseTemp` (`.WhiteTemp` (break `PostProcessSettings` (`PostProcessVolume.Settings` _output_get))))
      (goto _label_4 :!via `Open`))))

(fn `UserConstructionScript`)