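; BP_Bait is a bait object that BP_Monster actors eat, after which it returns to its starting location.
; Overlaps on SphereChow count monsters in range and start a ChowTimer countdown on Tick, which resets once all have left.
; At zero, physics and collision switch off for the move to the saved spawn point, then switch back on.
; Pickup respawn and AI sight-stimulus toggling nodes exist but are disconnected.
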(event `self.ReceiveBeginPlay`
  (set `self.SpawnPos` (`self.K2_GetActorLocation`)))

(event `self.SphereChow.OnComponentBeginOverlap`
  (params (OverlappedComponent :type "PrimitiveComponent Object Reference") (OtherActor :type "Actor Object Reference") (OtherComp :type "PrimitiveComponent Object Reference") (OtherBodyIndex :type Integer) (bFromSweep :type Boolean) (SweepResult :type "HitResult Structure (by ref)"))
  (cast `/Game/GraveyardShift/Characters/Undead/Monster/BP_Monster` OtherActor)
  (bind _result (`/Engine/EditorBlueprintResources/StandardMacros.IncrementInt` (`self.MonstersInRange`))
    (:`  `
      (set `self.bIsBeingEaten` true)
      (if (== _result 1)
        (set `self.TimeUntilEaten` (`self.ChowTimer`))))))

(event `self.SphereChow.OnComponentEndOverlap`
  (params (OverlappedComponent :type "PrimitiveComponent Object Reference") (OtherActor :type "Actor Object Reference") (OtherComp :type "PrimitiveComponent Object Reference") (OtherBodyIndex :type Integer))
  (bind _mesh (`self.Mesh`))
  (cast `/Game/GraveyardShift/Characters/Undead/Monster/BP_Monster` OtherActor)
  (`KismetSystemLibrary.PrintString` "Hello" true true (struct :`R` 0.021506 :`G` 1.0 :`A` 1.0))
  (bind _result (`/Engine/EditorBlueprintResources/StandardMacros.DecrementInt` (`self.MonstersInRange`))
    (:`  `
      (if (== _result 0)
        (set `self.bIsBeingEaten` false :!label _label)
        (set `self.TimeUntilEaten` (`self.ChowTimer`))
        (set `self.MonstersInRange` 0)
        (`PrimitiveComponent.SetCollisionEnabled` (`self.Mesh`) "QueryAndPhysics")
        (`PrimitiveComponent.SetSimulatePhysics` _mesh true)
        (`PrimitiveComponent.SetEnableGravity` _mesh true)))))

(event `self.ReceiveTick`
  (params (DeltaSeconds :type "Float (single-precision)"))
  (bind _mesh (`self.Mesh`))
  (if (`self.bIsBeingEaten`)
    (bind _output_get (set `self.TimeUntilEaten` (- (`self.TimeUntilEaten`) DeltaSeconds)))
    (if (<= _output_get 0.0)
      (`PrimitiveComponent.SetSimulatePhysics` _mesh false)
      (`PrimitiveComponent.SetEnableGravity` _mesh false)
      (`PrimitiveComponent.SetCollisionEnabled` (`self.Mesh`) "NoCollision")
      (`self.K2_SetActorLocation` (`self.SpawnPos`) true)
      (goto _label))))

(fn `UserConstructionScript`)