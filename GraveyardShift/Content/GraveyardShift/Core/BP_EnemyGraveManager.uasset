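; Graveyard enemy manager that repeatedly spawns random enemies from random free BP_Grave actors on a looping timeline.
; SpawnEnemy passes exit targets to each enemy and tints it and its grave with a shared random color through BP_ColorIdentifier.
; Graves move between available and in-use lists, returning on their OnReset event, which also decrements the active count.
; An active-enemy cap check exists but is unconnected, so only free graves limit spawning.
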(event `self.ReceiveBeginPlay`
  (`|ExecutionSequence`
    (:`then_0`
      (bind _outactors (`GameplayStatics.GetAllActorsOfClass` "/Game/GraveyardShift/Core/BP_Grave.BP_Grave_C"))
      (set `self.AvailableGraves` _outactors))
    (:`then_1`
      (for _array_element (`self.AvailableGraves`)
        (add `/Game/GraveyardShift/Core/BP_Grave.OnReset` _array_element (delegate `OnGraveReset_Event`)))
      (`Timeline|Timeline_EnemySpawn` :`NewTime` 5.0 :!via `PlayFromStart` :!label _label
        (:`Finished`
          (`KismetSystemLibrary.PrintString` "Spawning")
          (`self.SpawnEnemy`)
          (goto _label :!via `PlayFromStart`))))))

(event `OnGraveReset_Event`
  (params (Grave :type "/Game/GraveyardShift/Core/BP_Grave Object Reference"))
  (bind _inusegraves (`self.InUseGraves`))
  (bind _returnvalue (`KismetArrayLibrary.Array_Find` (`self.InUseGraves`) Grave))
  (bind _output (`|GetArrayItem` _inusegraves _returnvalue))
  (if (!= _returnvalue -1)
    (`KismetArrayLibrary.Array_Add` (`self.AvailableGraves`) _output)
    (`KismetArrayLibrary.Array_RemoveItem` _inusegraves _output)
    (`/Engine/EditorBlueprintResources/StandardMacros.DecrementInt` (`self.ActiveEnemies`))
    (else
      (`KismetSystemLibrary.PrintString` "RETURNING GRAVE ERROR" true true (struct :`R` 1.0 :`B` 0.007542 :`A` 1.0) 5.0))))

(fn `SpawnEnemy`
  (locals (CurrentGrave :type "/Game/GraveyardShift/Core/BP_Grave Object Reference") (CurrentEColor :type "/Game/GraveyardShift/Core/E_Colors Enum"))
  (bind _currentgrave (`local.CurrentGrave`))
  (bind _currentecolor (`local.CurrentEColor`))
  (bind _colorvalues_colorvalues (break `/Game/GraveyardShift/Core/S_Colors` (`self.ColorValues`)))
  (bind _colorvalues_colorvalues_2 (break `/Game/GraveyardShift/Core/S_Colors` (`self.ColorValues`)))
  (bind _availablegraves (`self.AvailableGraves`))
  (bind _value (`BlueprintMapLibrary.Map_Find` _colorvalues_colorvalues_2 _currentecolor))
  (bind _returnvalue (`self.GetComponentByClass` (`local.CurrentGrave`) "/Game/GraveyardShift/Core/BP_ColorIdentifier.BP_ColorIdentifier_C"))
  (bind _returnvalue_2 (cast `/Game/GraveyardShift/Core/E_Colors` (`KismetMathLibrary.Conv_IntToByte` (`KismetMathLibrary.RandomInteger` (enumcount `/Game/GraveyardShift/Core/E_Colors`)))))
  (set `local.CurrentEColor` _returnvalue_2)
  (if (`.ReturnValue` (`BlueprintMapLibrary.Map_Find` _colorvalues_colorvalues _returnvalue_2))
    (if (`KismetArrayLibrary.Array_IsNotEmpty` (`self.EnemyBlueprints`))
      (if (`KismetArrayLibrary.Array_IsNotEmpty` _availablegraves)
        (bind _output_get (set `local.CurrentGrave` (`KismetArrayLibrary.Array_Random` _availablegraves)))
        (bind (_returnvalue_location _returnvalue_rotation) (`KismetMathLibrary.BreakTransform` (`self.GetTransform` _output_get)))
        (bind _returnvalue_3 (`|SpawnActorFromClass` (`GameplayStatics.GetObjectClass` (`KismetArrayLibrary.Array_Random` (`self.EnemyBlueprints`))) (`KismetMathLibrary.MakeTransform` (+ _returnvalue_location (0.0 0.0 70.0)) _returnvalue_rotation) "AlwaysSpawn" "MultiplyWithRoot" null null))
        (`/Engine/EditorBlueprintResources/StandardMacros.IsValid` _returnvalue_3
          (:`Is Valid`
            (set `/Game/GraveyardShift/Characters/Monsters/BP_Monster.ExitTargets` (`self.ExitTargets`) _returnvalue_3)
            (bind _returnvalue_4 (`self.GetComponentByClass` _returnvalue_3 "/Game/GraveyardShift/Core/BP_ColorIdentifier.BP_ColorIdentifier_C"))
            (set `/Game/GraveyardShift/Core/BP_ColorIdentifier.Color` _currentecolor _returnvalue_4)
            (`/Game/GraveyardShift/Core/BP_ColorIdentifier.SetMatColor` _returnvalue_4 _value)
            (set `/Game/GraveyardShift/Core/BP_ColorIdentifier.Color` _currentecolor _returnvalue)
            (`/Game/GraveyardShift/Core/BP_ColorIdentifier.SetMatColor` _returnvalue _value)
            (`KismetArrayLibrary.Array_Add` (`self.InUseGraves`) _currentgrave)
            (bind _returnvalue_5 (`KismetArrayLibrary.Array_RemoveItem` (`self.AvailableGraves`) _currentgrave))
            (if _returnvalue_5
              (`/Engine/EditorBlueprintResources/StandardMacros.IncrementInt` (`self.ActiveEnemies`))
              (else
                (`KismetSystemLibrary.PrintString` "GRAVE LIST ERROR"))))
          (:`Is Not Valid`
            (`KismetSystemLibrary.PrintString` "SPAWN ERROR")))
        (else
          (`KismetSystemLibrary.PrintString` "NoAvailableGraves")))
      (else
        (`KismetSystemLibrary.PrintString` "ENEMY BPArr ERROR")))
    (else
      (`KismetSystemLibrary.PrintString` "COLOR FINDING ERROR"))))

(fn `UserConstructionScript`)