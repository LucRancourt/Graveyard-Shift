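; BP_Exit is a gate exit that plays an escalating escape sequence while monsters occupy its box trigger, ending in a printed "Game Over!".
; The first overlapping BP_Monster starts the sequence, and each sound's finish event advances it through latch, rattling and opening.
; An overlap counter resets the step and stops the audio when the last monster leaves.
; An older per-monster timer approach remains as disconnected nodes.
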(event `PlayAudioSequence`
  (switch `int` (`self.ExitPhaseStep`)
    (:`0`
      (set `self.CurrentSound` "/Game/GraveyardShift/Audio/SFX/SC_Gate_Latch.SC_Gate_Latch")
      (bind _returnvalue (`GameplayStatics.SpawnSoundAtLocation` (`self.CurrentSound`) (`self.K2_GetActorLocation`) (struct) 1.0 1.0 0.0 null null :!label _label))
      (bind _output_get (set `self.CurrentSoundSource` _returnvalue))
      (`/Engine/EditorBlueprintResources/StandardMacros.IncrementInt` (`self.ExitPhaseStep`)
        (:`  `
          (add `AudioComponent.OnAudioFinished` _output_get (delegate `PlayAudioSequence`)))))
    (:`1`
      (set `self.CurrentSound` "/Game/GraveyardShift/Audio/SFX/SC_Gate_Rattling.SC_Gate_Rattling")
      (goto _label))
    (:`2`
      (set `self.CurrentSound` "/Game/GraveyardShift/Audio/SFX/SC_Gate_Rattling.SC_Gate_Rattling")
      (goto _label))
    (:`3`
      (set `self.CurrentSound` "/Game/GraveyardShift/Audio/SFX/SC_Gate_Opening.SC_Gate_Opening")
      (goto _label))
    (:`4`
      (`KismetSystemLibrary.PrintString` "Game Over!" true true (struct :`R` 1.0 :`G` 0.009899 :`A` 1.0) 10.0))))

(event `self.Box.OnComponentBeginOverlap`
  (params (OverlappedComponent :type "PrimitiveComponent Object Reference") (OtherActor :type "Actor Object Reference") (OtherComp :type "PrimitiveComponent Object Reference") (OtherBodyIndex :type Integer) (bFromSweep :type Boolean) (SweepResult :type "HitResult Structure (by ref)"))
  (cast `/Game/GraveyardShift/Characters/Monsters/BP_Monster` OtherActor)
  (bind _result (`/Engine/EditorBlueprintResources/StandardMacros.IncrementInt` (`self.OverlappingMon`))
    (:`  `
      (if (== _result 1)
        (`self.PlayAudioSequence`)))))

(event `self.Box.OnComponentEndOverlap`
  (params (OverlappedComponent :type "PrimitiveComponent Object Reference") (OtherActor :type "Actor Object Reference") (OtherComp :type "PrimitiveComponent Object Reference") (OtherBodyIndex :type Integer))
  (bind _currentsoundsource (`self.CurrentSoundSource`))
  (cast `/Game/GraveyardShift/Characters/Monsters/BP_Monster` OtherActor)
  (bind _result (`/Engine/EditorBlueprintResources/StandardMacros.DecrementInt` (`self.OverlappingMon`))
    (:`  `
      (if (<= _result 0)
        (`|ExecutionSequence`
          (:`then_0`
            (set `self.ExitPhaseStep` 0))
          (:`then_1`
            (`/Engine/EditorBlueprintResources/StandardMacros.IsValid` _currentsoundsource
              (:`Is Valid`
                (clear `AudioComponent.OnAudioFinished` _currentsoundsource)
                (`AudioComponent.Stop` _currentsoundsource)
                (`ActorComponent.K2_DestroyComponent` _currentsoundsource))))
          (:`then_2`
            (set `self.CurrentSoundSource` null)))))))

(event `self.ReceiveTick`
  (params (DeltaSeconds :type "Float (single-precision)"))
  (set `self.Delta Seconds` DeltaSeconds))

(fn `UserConstructionScript`)