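; First-person player character that carries pickups and relays win, damage and loss feedback in a ghost-themed game.
; A camera trace each tick highlights pickups via an outline post-process; Interact picks up, uses the Interacter or drops, recording the held item's desired or feared identifier.
; The ghost counter's all-removed event and damage drive the Flash widget, whose callbacks fire delayed win/loss dispatchers.
; Freeze temporarily disables input.
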(event `PlayerWon`
  (`KismetSystemLibrary.Delay` 2.0)
  (`self.OnWin`))

(event `PlayerWin`
  (`/Game/GraveyardShift/Core/TempScreenFlash/WBP_Flash.FadeInOut` (`self.Flash`) true true))

(event `PlayerDamage`
  (params (IsDead :type Boolean))
  (`/Game/GraveyardShift/Core/TempScreenFlash/WBP_Flash.FadeInOut` (`self.Flash`) IsDead false))

(event `PlayerIsDead`
  (`KismetSystemLibrary.Delay` 2.0)
  (`self.OnLoss`))

(event `self.ReceiveBeginPlay`
  (bind _returnvalue (`GameplayStatics.GetActorOfClass` "/Game/GraveyardShift/Core/BP_GhostCounter.BP_GhostCounter_C"))
  ; Comment
  (`/Engine/EditorBlueprintResources/StandardMacros.IsValid` _returnvalue
    (:`Is Valid`
      (add `/Game/GraveyardShift/Core/BP_GhostCounter.OnAllGhostRemoved` _returnvalue (delegate `PlayerWin`))
      (`/MyInteractSystem/BPFL_InteractSystem.SetPostProcessForOutline` (`self.FPCameraComponent`) "/MyInteractSystem/MaterialLibrary/Outline/M_Outline.M_Outline")
      (bind _returnvalue_2 (`|CreateWidget` "/Game/GraveyardShift/Core/TempScreenFlash/WBP_Flash.WBP_Flash_C" (`GameplayStatics.GetPlayerController` 0)))
      (bind _output_get (set `self.Flash` _returnvalue_2))
      (`UserWidget.AddToViewport` _output_get 0)
      (add `/Game/GraveyardShift/Core/TempScreenFlash/WBP_Flash.PlayerDied` _output_get (delegate `PlayerIsDead`))
      (add `/Game/GraveyardShift/Core/TempScreenFlash/WBP_Flash.PlayerWon` _output_get (delegate `PlayerWon`)))))

(event `EnhancedInput|/Game/GraveyardShift/Core/Input/InputActions/IA_Interact`
  (params (ActionValue :type Boolean) (ElapsedSeconds :type "Float (double-precision)") (TriggeredSeconds :type "Float (double-precision)") (InputAction :type "InputAction Object Reference" :default "/Game/GraveyardShift/Core/Input/InputActions/IA_Interact.IA_Interact"))
  (bind _pickupinview (`self.PickupInView`))
  (bind _returnvalue (`SceneComponent.K2_GetComponentLocation` (`self.FPCameraComponent`)))
  (bind _desiredobjectidentifier (`/Game/GraveyardShift/Core/Interactable/BP_Pickup.DesiredObjectIdentifier` _pickupinview))
  (bind _fearedobjectidentifier (`/Game/GraveyardShift/Core/Interactable/BP_Pickup.FearedObjectIdentifier` _pickupinview))
  (:`Started`
    (`/Engine/EditorBlueprintResources/StandardMacros.IsValid` (`self.HeldPickup`)
      (:`Is Valid`
        (bind (_outhit _returnvalue_2) (`KismetSystemLibrary.LineTraceSingle` _returnvalue (+ (* (`SceneComponent.GetForwardVector` (`self.FPCameraComponent`)) 300.0) _returnvalue) "TraceTypeQuery1"))
        (if _returnvalue_2
          (bind (_bblockinghit _binitialoverlap _time _distance _location _impactpoint _normal _impactnormal _physmat _hitactor) (`GameplayStatics.BreakHitResult` _outhit))
          (cast `InteractableActor` _hitactor
            (:`then`
              (`InteracterComponent.TryInteract` (`self.Interacter`) :!label _label))
            (:`CastFailed`
              (`/Engine/EditorBlueprintResources/StandardMacros.IsValid` (`self.GetComponentByClass` _hitactor "/Script/MyInteractSystem.InteractableComponent")
                (:`Is Valid`
                  (goto _label))
                (:`Is Not Valid`
                  (`self.DropPickup` :!label _label_2)))))
          (else
            (goto _label_2))))
      (:`Is Not Valid`
        (`/Engine/EditorBlueprintResources/StandardMacros.IsValid` _pickupinview
          (:`Is Valid`
            (if (`|EnumInequality` _desiredobjectidentifier "NewEnumerator1")
              (set `self.HeldItemEnum` _desiredobjectidentifier)
              (bind _output_get (set `self.HeldPickup` (`self.PickupInView`) :!label _label_3))
              (set `self.PickupInView` null)
              (`/Game/GraveyardShift/Core/Interactable/BP_Pickup.Pickup` _output_get null (`self.FPCameraComponent`))
              (elif (`|EnumInequality` _fearedobjectidentifier "NewEnumerator1")
                (set `self.HeldItemEnum` _fearedobjectidentifier)
                (goto _label_3))))
          (:`Is Not Valid`
            (goto _label)))))))

(event `Freeze`
  (params (Duration :type "Float (double-precision)"))
  (bind _returnvalue (`GameplayStatics.GetPlayerController` 0))
  (`self.DisableInput` _returnvalue)
  (`KismetSystemLibrary.Delay` Duration)
  (`self.EnableInput` _returnvalue))

(event `self.ReceiveTick`
  (params (DeltaSeconds :type "Float (single-precision)"))
  (bind _pickupinview (`self.PickupInView`))
  (bind _returnvalue (`SceneComponent.K2_GetComponentLocation` (`self.FPCameraComponent`)))
  (`/Engine/EditorBlueprintResources/StandardMacros.IsValid` _pickupinview
    (:`Is Valid`
      (`/Game/GraveyardShift/Core/Interactable/BP_Pickup.Highlight` _pickupinview false))
    (:`Is Not Valid`
      _))
  (bind (_outhit _returnvalue_2) (`KismetSystemLibrary.LineTraceSingle` _returnvalue (+ (* (`SceneComponent.GetForwardVector` (`self.FPCameraComponent`)) 300.0) _returnvalue) "TraceTypeQuery1"))
  (if _returnvalue_2
    (bind _asbp_pickup (cast `/Game/GraveyardShift/Core/Interactable/BP_Pickup` (`.HitActor` (`GameplayStatics.BreakHitResult` _outhit))))
    (bind _output_get (set `self.PickupInView` _asbp_pickup))
    (`/Game/GraveyardShift/Core/Interactable/BP_Pickup.Highlight` _output_get true)))

(fn `DropPickup`
  (`/Game/GraveyardShift/Core/Interactable/BP_Pickup.Drop` (`self.HeldPickup`))
  (set `self.HeldPickup` null)
  (set `self.HeldItemEnum` 0))

(fn `UserConstructionScript`)