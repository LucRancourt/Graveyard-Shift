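; Sprite-based pickup actor that can be held, dropped and highlighted.
; While not held, Tick yaw-billboards the sprite to the camera and snaps the actor onto the surface below with a downward trace.
; Pickup disables collision and attaches it at half scale to a holder actor or component; Drop detaches it and restores scale and collision.
; Highlighting toggles custom depth with a stencil value, and sounds play on pickup and drop.
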(event `self.ReceiveBeginPlay`
  (set `self.InitialScale` (`self.GetActorRelativeScale3D`))
  (set `SceneComponent.bAbsoluteRotation` true (`self.Sprite`)))

(event `self.ReceiveTick`
  (params (DeltaSeconds :type "Float (single-precision)"))
  (bind _returnvalue (`self.K2_GetActorLocation`))
  (bind (_min _max) (`StaticMeshComponent.GetLocalBounds` (`self.Sprite`)))
  (if (not (`self.IsHeld`))
    (`self.YawBillboarding`)
    (bind (_outhit _returnvalue_2) (`KismetSystemLibrary.LineTraceSingle` _returnvalue (- _returnvalue (* (`KismetMathLibrary.Vector_Up`) 10000.0)) "TraceTypeQuery3"))
    (if _returnvalue_2
      (`self.K2_SetActorLocation` (+ (`.Location` (`GameplayStatics.BreakHitResult` _outhit)) (`KismetMathLibrary.MakeVector` 0.0 0.0 (`KismetMathLibrary.SafeDivide` (+ (`KismetMathLibrary.Abs` (.x _min)) (`KismetMathLibrary.Abs` (.x _max))) 2.0)))))
    (set `self.IsHeld` false :!label _label)))

(event `Pickup`
  (params (Holder :type "Actor Object Reference") (HolderComp :type "SceneComponent Object Reference"))
  (if (not (`self.IsHeld`))
    (set `self.IsHeld` true)
    (`self.Highlight` false)
    (`GameplayStatics.PlaySound2D` "/Game/GraveyardShift/Audio/SFX/SC_Pickup_Pickup.SC_Pickup_Pickup" 1.0 1.0 0.0 null null)
    (`PrimitiveComponent.SetCollisionEnabled` (`self.Sprite`) "NoCollision")
    (`KismetSystemLibrary.Delay` 0.01)
    (`/Engine/EditorBlueprintResources/StandardMacros.IsValid` Holder
      (:`Is Valid`
        (set `SceneComponent.bAbsoluteRotation` false (`self.Sprite`))
        (`self.K2_AttachToActor` Holder "None" "KeepRelative" "KeepRelative" "KeepRelative" false))
      (:`Is Not Valid`
        (`/Engine/EditorBlueprintResources/StandardMacros.IsValid` HolderComp
          (:`Is Valid`
            (set `SceneComponent.bAbsoluteRotation` false (`self.Sprite`))
            (`self.K2_AttachToComponent` HolderComp "None" "KeepRelative" "KeepRelative" "KeepRelative" false)))))
    (`self.K2_SetActorRelativeLocation` (`self.HoldOffset`))
    (`self.SetActorRelativeScale3D` (/ (`self.InitialScale`) 2.0))
    (`self.K2_SetActorRelativeRotation` (struct :`Yaw` -90.0 :`Roll` 90.0))))

(event `Drop`
  (if (`self.IsHeld`)
    (`self.Highlight` false)
    (`GameplayStatics.PlaySound2D` "/Game/GraveyardShift/Audio/SFX/SC_Pickup_Drop.SC_Pickup_Drop" 1.0 1.0 0.0 null null)
    (`self.SetActorRelativeScale3D` (`self.InitialScale`))
    (`self.K2_DetachFromActor` "KeepWorld" "KeepWorld")
    (`PrimitiveComponent.SetCollisionEnabled` (`self.Sprite`) "QueryAndPhysics")
    (goto _label)))

(event `Highlight`
  (params (IsEnabled :type Boolean))
  (`PrimitiveComponent.SetRenderCustomDepth` (`self.Sprite`) IsEnabled))

(event `DisablePickup`
  (`PrimitiveComponent.SetCollisionEnabled` (`self.Sprite`) "NoCollision"))

(event `EnablePickup`
  (`PrimitiveComponent.SetCollisionEnabled` (`self.Sprite`) "QueryAndPhysics"))

(fn `UserConstructionScript`
  (bind _sprite (`self.Sprite`))
  (`PrimitiveComponent.SetRenderInDepthPass` _sprite true)
  (`PrimitiveComponent.SetCustomDepthStencilValue` _sprite 1))

(fn `YawBillboarding`
  (bind (_returnvalue_roll _returnvalue_pitch _returnvalue_yaw) (`KismetMathLibrary.BreakRotator` (`KismetMathLibrary.FindLookAtRotation` (`SceneComponent.K2_GetComponentLocation` (`self.Sprite`)) (`PlayerCameraManager.GetCameraLocation` (`GameplayStatics.GetPlayerCameraManager` 0)))))
  (`SceneComponent.K2_SetWorldRotation` (`self.Sprite`) (`KismetMathLibrary.MakeRotator` 90.0 0.0 (- _returnvalue_yaw 90.0)) false false))