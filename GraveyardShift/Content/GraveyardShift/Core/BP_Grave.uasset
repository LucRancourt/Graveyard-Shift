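; BP_Grave is a color-coded grave that takes back a BP_Monster of the same color.
; A matching monster leaving InitialOverlapBox arms the grave by setting IsActive.
; While armed, a matching monster entering Box is destroyed, then the grave disarms, resets its identifier's material color and fires the OnReset dispatcher.
; Both overlap events share the ColorCheck macro, which compares the monster's and grave's BPColorIdentifier colors.
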(event `self.Box.OnComponentBeginOverlap`
  (params (OverlappedComponent :type "PrimitiveComponent Object Reference") (OtherActor :type "Actor Object Reference") (OtherComp :type "PrimitiveComponent Object Reference") (OtherBodyIndex :type Integer) (bFromSweep :type Boolean) (SweepResult :type "HitResult Structure (by ref)"))
  (if (`self.IsActive`)
    (bind _asbp_monster (cast `/Game/GraveyardShift/Characters/Monsters/BP_Monster` OtherActor))
    (`self.ColorCheck` _asbp_monster
      (:`true`
        (set `self.IsActive` false)
        (`self.K2_DestroyActor` _asbp_monster)
        (set `self.IsActive` false)
        (`/Game/GraveyardShift/Core/BP_ColorIdentifier.ResetMatColor` (`self.BP_ColorIdentifier`))
        (`self.OnReset` self)))))

(event `self.InitialOverlapBox.OnComponentEndOverlap`
  (params (OverlappedComponent :type "PrimitiveComponent Object Reference") (OtherActor :type "Actor Object Reference") (OtherComp :type "PrimitiveComponent Object Reference") (OtherBodyIndex :type Integer))
  (bind _asbp_monster (cast `/Game/GraveyardShift/Characters/Monsters/BP_Monster` OtherActor))
  (`self.ColorCheck` _asbp_monster
    (:`true`
      (set `self.IsActive` true))))

(fn `UserConstructionScript`)