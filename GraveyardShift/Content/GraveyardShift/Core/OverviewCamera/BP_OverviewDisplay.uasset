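; BP_OverviewDisplay is an interactable screen that shows camera views, cycling to the next one each time it is used.
; On BeginPlay it creates a dynamic instance of the render-target material M_RTCameraViews on its static mesh and checks that the camera texture list is non-empty.
; Interact advances a wrapping index and sets that texture as the material's CameraView parameter, while CanInteract always allows interaction.
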(event `self.ReceiveBeginPlay`
  (bind _returnvalue (`PrimitiveComponent.CreateDynamicMaterialInstance` (`self.StaticMesh`) 0 "/Game/GraveyardShift/MaterialLibrary/RenderTargets/M_RTCameraViews.M_RTCameraViews" "None"))
  (set `self.DynaMaterialInst` _returnvalue)
  (set `self.bIsCameraViewTextureListValid` (> (`KismetArrayLibrary.Array_Length` (`self.CameraViewTextureList`)) 0)))

(event `MyInteractableInterface.Interact`
  (params (Interactor :type "Actor Object Reference"))
  (bind _currentcameraindex (`self.CurrentCameraIndex`))
  (bind _cameraviewtexturelist (`self.CameraViewTextureList`))
  (if (`self.bIsCameraViewTextureListValid`)
    (`|ExecutionSequence`
      (:`then_0`
        (bind _result (`/Engine/EditorBlueprintResources/StandardMacros.IncrementInt` _currentcameraindex)
          (:`  `
            (if (>= _result (`KismetArrayLibrary.Array_Length` _cameraviewtexturelist))
              (set `self.CurrentCameraIndex` 0)))))
      (:`then_1`
        (bind _output_get (set `self.CurrentCameraViewTexture` (`|GetArrayItem` _cameraviewtexturelist _currentcameraindex)))
        (`MaterialInstanceDynamic.SetTextureParameterValue` (`self.DynaMaterialInst`) "CameraView" _output_get)))))

(fn `CanInteract`
  (params (Interactor :type "Actor Object Reference"))
  (returns (ReturnValue :type Boolean))
  (return true))

(fn `UserConstructionScript`)